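; Lava particle Blueprint that repeatedly emits LavaEmbers effects at the location and rotation of its ParticleSystem component.
; Tick calls Spawn and Despawn every frame, relying on their Delay nodes to pace them on separate timers.
; Spawn creates an emitter with a heavily increased custom time dilation.
; Despawn destroys only the most recently spawned emitter, on a slightly longer cycle than spawning.
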(event Custom|Spawn
  (bind _particlesystem (Variables|Default|GetParticleSystem))
  (Utilities|FlowControl|Delay 2.0)
  (bind _returnvalue (Effects|SpawnEmitteratLocation "/Game/Blueprints/Etc/LavaEmbers.LavaEmbers" (Transformation|GetWorldLocation _particlesystem) (Transformation|GetWorldRotation _particlesystem)))
  (Variables|/Script/Engine.ParticleSystemComponent|SetCustomTimeDilation _returnvalue 65.0))

(event Custom|Despawn
  (Utilities|FlowControl|Delay 3.0)
  (Components|DestroyComponent (stale Custom|Spawn _returnvalue)))

(event EventTick
  (params (DeltaSeconds :type Float%20%28single-precision%29))
  (CallFunction|Spawn)
  (CallFunction|Despawn))

(fn ConstructionScript)