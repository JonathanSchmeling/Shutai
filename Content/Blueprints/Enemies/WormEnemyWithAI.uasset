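; Worm enemy for a side-scroller that damages the player on sight and can be killed with the sword.
; BeginPlay caches the player, sword and Varis game instance; sword overlaps during a swing reduce Health.
; Pawn sensing fires a targetless AIMoveTo and calls the player's TakeDamage immediately and again on success.
; Tick destroys the worm at zero Health and records it in Varis.DestroyedActors; older tiered health-bar damage logic remains disconnected.
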(event OnSeePawn(PawnSensing)
  (params (Pawn :type Pawn%20Object%20Reference))
  ;[1 1 1] AI
  (AI|AIMoveTo self "0, 0, 0" 0 5.0 false
    (:then
      _)
    (:OnSuccess
      _))
  (CallFunction|Attack))

(event Custom|Attack
  ;[1 1 1] Attack
  (Default|TakeDamage (Variables|Default|GetMy%20character)))

(event Custom|OnActorBeginOverlap_Event_0
  (params (OverlappedActor :type Actor%20Object%20Reference) (OtherActor :type Actor%20Object%20Reference))
  ;[1 1 1] Attack
)

(event EventTick
  (params (DeltaSeconds :type Float%20%28single-precision%29))
  ;[1 1 1] Death
  (if (<= (Variables|Default|GetHealth) 0.0)
    (Actor|DestroyActor)
    (Variables|Default|SetIsDestroyed? true)
    (Utilities|Array|Add (Variables|/Game/Blueprints/Player/Varis.Varis_C|GetDestroyed%20Actors (stale EventBeginPlay _output_get)) self)))

(event EventBeginPlay
  ;[1 1 1] Variables
  (bind _outactors (Actor|GetAllActorsOfClass "/Game/Blueprints/Player/SideScrollerCharacter.SideScrollerCharacter_C"))
  (for _array_element _outactors
    (Variables|Default|SetMy%20character _array_element)
    (bind _outactors_2 (Actor|GetAllActorsOfClass "/Game/Blueprints/Sword/MySwordBP.MySwordBP_C"))
    (for _array_element_2 _outactors_2
      (bind _asmy_sword_bp (Utilities|Casting|CastToMySwordBP _array_element_2))
      (Variables|Default|SetMySword _asmy_sword_bp)
      (bind _asvaris (Utilities|Casting|CastToVaris (Game|GetGameInstance)))
      (bind _output_get (Variables|Default|SetVaris _asvaris)))))

(event Collision|EventActorBeginOverlap
  (params (OtherActor :type Actor%20Object%20Reference))
  (bind _my_character (Variables|Default|GetMy%20character))
  (bind _mysword (Variables|Default|GetMySword))
  ;[1 1 1] Take Damage
  (if (Utilities|IsValid _my_character)
    (if (Variables|/Game/Blueprints/Player/SideScrollerCharacter.SideScrollerCharacter_C|GetIsSwinging? _my_character)
      (for _array_element (Collision|GetOverlappingActors (Utilities|GetClass _mysword) :!class /Script/Engine.Actor)
        (Game|Damage|ApplyDamage self 0.0 0 0)
        (Variables|Default|SetDamage%20Taken? true)
        (Variables|Default|SetHealth (- (Variables|Default|GetHealth) (Variables|/Game/Blueprints/Sword/MySwordBP.MySwordBP_C|GetDamage _mysword)))))))

(fn ConstructionScript)