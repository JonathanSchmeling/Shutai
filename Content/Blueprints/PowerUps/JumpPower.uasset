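; JumpPower is a pickup actor that upgrades the player's jump count and moves them to the Lava_World level.
; On BeginPlay it caches the player's SideScrollerCharacter.
; When that character overlaps it, it destroys itself, sets PlayerJumpCt on the Varis game instance to grant a double jump, then opens Lava_World with an Inferno_Burrower PlayerStart option.
; Storing the count on the game instance carries it across the level load.
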(event Collision|EventActorBeginOverlap
  (params (OtherActor :type Actor%20Object%20Reference))
  (if (Collision|IsOverlappingActor (stale EventBeginPlay _asside_scroller_character) :!class /Script/Engine.Actor)
    (Actor|DestroyActor)
    (bind _asvaris (Utilities|Casting|CastToVaris (Game|GetGameInstance)))
    (Variables|/Game/Blueprints/Player/Varis.Varis_C|SetPlayerJumpCt _asvaris 2)
    (Game|OpenLevel(byName) "Lava_World" true "PlayerStart: Inferno_Burrower")))

(event EventBeginPlay
  (bind _asside_scroller_character (Utilities|Casting|CastToSideScrollerCharacter (Game|GetPlayerCharacter 0)))
  (Variables|Default|SetCharacter _asside_scroller_character))

(fn ConstructionScript)