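; Varis is a player Blueprint that, on Init, applies a double jump and saves to a slot.
; Init creates a base SaveGame object, then, if PlayerJumpCt equals two, sets the SideScrollerCharacter's JumpMaxCount to match.
; It then writes that object to a fixed-name slot and prints a confirmation, without copying any values into the save or loading one.
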(event EventInit
  (bind _returnvalue (SaveGame|CreateSaveGameObject "/Script/Engine.SaveGame"))
  (if (== (Variables|Default|GetPlayerJumpCt) 2)
    (bind _asside_scroller_character (Utilities|Casting|CastToSideScrollerCharacter (Game|GetPlayerCharacter 0)))
    (Variables|/Script/Engine.Character|SetJumpMaxCount _asside_scroller_character 2)
    (bind _output_get (Variables|Default|SetPlayerName "PlayerName"))
    (SaveGame|SaveGametoSlot _returnvalue _output_get (Variables|Default|GetUserIndex))
    (Development|PrintString "Game Saved")))